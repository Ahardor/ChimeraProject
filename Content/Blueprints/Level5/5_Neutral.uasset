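; Level 5 neutralization container, a child Blueprint that simulates tilt-based pouring and acid-base indicator color.
; Spill replaces the parent version, scaling Niagara particles, spill point and drain rate by angle, draining compounds evenly and hiding the liquid mesh when empty.
; ComputeColor uses Indicator, NaOH and HCl presence, sampling a color curve by their amount difference when all three are mixed.
; Tick and AddFill defer to the parent.
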(event EventBeginPlay
  (|CallParentFunction) ; This node is disabled and will not be called.\nDrag off pins to build functionality.
)

(event Collision|EventActorBeginOverlap
  (params (OtherActor :type Actor%20Object%20Reference))
  (|CallParentFunction OtherActor) ; This node is disabled and will not be called.\nDrag off pins to build functionality.
)

(event EventTick
  (params (DeltaSeconds :type Float%20%28single-precision%29))
  (|CallParentFunction DeltaSeconds))

(fn ConstructionScript
  (|CallParentFunction))

(fn Spill
  (bind _compound (Variables|Default|GetCompound))
  (bind _minspillrate (Variables|Default|GetMinSpillRate))
  (bind _maxspillrate (Variables|Default|GetMaxSpillRate))
  (bind _angle (Variables|Default|GetAngle))
  (bind _niagara (Variables|Default|GetNiagara))
  (bind _returnvalue (Math|Float|Absolute(Float) _angle))
  (bind _returnvalue_2 (/ _returnvalue 9e+01))
  (bind _returnvalue_3 (Math|Float|Lerp _minspillrate _maxspillrate _returnvalue_2))
  (if (!= (Variables|Default|GetFill) 0.0)
    (Effects|Components|ParticleSystem|SetFloatParameter _niagara "SpawnRate" (Math|Float|Lerp 1e+01 (* (Variables|Default|GetMaxSpillRadius) 3e+03) _returnvalue_2))
    (Effects|Components|ParticleSystem|SetFloatParameter _niagara "SpawnRadius" (Math|Float|Lerp 0.2 (Variables|Default|GetMaxSpillRadius) _returnvalue_2))
    (bind _output_get (Variables|Default|SetSpillPoint (Math|Vector|Lerp(Vector) (Transformation|GetWorldLocation (Variables|Default|GetParticleInit)) (- (/ (+ (Transformation|GetWorldLocation (Variables|Default|GetCube1)) (Transformation|GetWorldLocation (Variables|Default|GetCube2))) 2.0) (Variables|Default|GetParticleOffset)) (Math|Float|Clamp(Float) (/ (- _returnvalue 9e+01) 9e+01)))))
    (Transformation|SetWorldLocation (Variables|Default|GetNiagara) _output_get false false)
    (bind _output_get_2 (Variables|Default|SetSpillRate _returnvalue_3))
    (bind _output_get_3 (Variables|Default|SetFill (Math|Float|Clamp(Float) (- (Variables|Default|GetFill) _returnvalue_3) 0.0 (Variables|Default|GetMaxFill))))
    (for (_ _array_index) _compound
      (Utilities|Struct|SetmembersinCompound (Utilities|Array|Get(acopy) _compound _array_index) (Math|Float|Clamp(Float) (- (.Amount (Utilities|Struct|BreakCompound (Utilities|Array|Get(acopy) _compound _array_index))) (/ _output_get_2 (Utilities|Array|Length _compound))) 0.0 (Variables|Default|GetMaxFill)))
      (if (== (Math|Float|Clamp(Float) (- (.Amount (Utilities|Struct|BreakCompound (Utilities|Array|Get(acopy) _compound _array_index))) (/ _output_get_2 (Utilities|Array|Length _compound))) 0.0 (Variables|Default|GetMaxFill)) 0.0)
        (Utilities|Array|RemoveIndex _compound _array_index)))
    (if (== _output_get_3 0.0)
      (Rendering|SetVisibility (Variables|Default|GetStaticMesh1) false false))))

(fn AddFill
  (params (Amount :type Float%20%28double-precision%29) (Comp :type Array%20of%20Compound%20Structures))
  (|CallParentFunction Amount Comp)
  (return))

(fn ComputeColor
  (bind _compound (Variables|Default|GetCompound))
  (bind (_find _item) (CallFunction|FindCompoundbyName _compound "HCl"))
  (bind (_find_2 _item_2) (CallFunction|FindCompoundbyName _compound "NaOH"))
  (bind (_find_3 _item_3) (CallFunction|FindCompoundbyName _compound "Indicator"))
  (if (and _find_2 _find)
    (Variables|Default|SetColor (select _find_3 (Math|Curves|GetLinearColorValue (Variables|Default|GetColorCurve) (+ (/ (.amount (Utilities|Array|Get(acopy) _compound _item_2)) 4e+01) (/ (.amount (Utilities|Array|Get(acopy) _compound _item)) -4e+01))) (Variables|Default|GetColor)))
    (else
      (Variables|Default|SetColor (select _find_3 (select _find_2 "(R=1.000000,G=0.756863,B=0.000000,A=0.411765)" (select _find "(R=1.000000,G=0.160784,B=0.533333,A=0.392157)" (.color (Utilities|Array|Get(acopy) _compound _item_3)))) (Variables|Default|GetColor))))))