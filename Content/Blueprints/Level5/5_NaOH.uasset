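; Level 5 sodium hydroxide (NaOH) container, a child Blueprint that reacts when an indicator compound is present in it.
; AddFill extends the parent fill logic: with an indicator present, it recolors that compound translucent amber, plays audio and, on the first occurrence, marks step 1 on the Tutorial widget.
; ComputeColor blends the current color toward the same amber by the indicator's share of the fill.
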(event EventBeginPlay
  (|CallParentFunction) ; This node is disabled and will not be called.\nDrag off pins to build functionality.
)

(event Collision|EventActorBeginOverlap
  (params (OtherActor :type Actor%20Object%20Reference)))

(event EventTick
  (params (DeltaSeconds :type Float%20%28single-precision%29))
  (|CallParentFunction DeltaSeconds) ; This node is disabled and will not be called.\nDrag off pins to build functionality.
)

(fn ConstructionScript
  (|CallParentFunction))

(fn AddFill
  (params (Amount :type Float%20%28double-precision%29) (Comp :type Array%20of%20Compound%20Structures))
  (bind _compound (Variables|Default|GetCompound))
  (bind (_find _item) (CallFunction|FindCompoundbyName _compound "Indicator"))
  (|CallParentFunction Amount Comp)
  (if _find
    (Utilities|Struct|SetmembersinCompound (Utilities|Array|Get(acopy) _compound _item) "(R=1.000000,G=0.756863,B=0.000000,A=0.411765)")
    (CallFunction|PlayAudio)
    (if (Variables|Default|GetAdded)
      _
      (else
        (Variables|Default|SetAdded true)
        (bind _foundwidgets (Widget|GetAllWidgetsOfClass "/Game/Blueprints/UI/Tutorial.Tutorial_C" true))
        (Class|StepCheckInterface|Mark(Message) (Utilities|Array|Get(acopy) _foundwidgets) 1 "NewEnumerator1")))
    (return)))

(fn ComputeColor
  (bind _compound (Variables|Default|GetCompound))
  (bind (_find _item) (CallFunction|FindCompoundbyName _compound "Indicator"))
  (if _find
    (Variables|Default|SetColor (Math|Color|Lerp(LinearColor) (Variables|Default|GetColor) "(R=1.000000,G=0.756725,B=0.000000,A=0.411000)" (/ (.Amount (Utilities|Struct|BreakCompound (Utilities|Array|Get(acopy) _compound _item))) (Variables|Default|GetFill))))))