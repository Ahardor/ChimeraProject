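; Touch player controller for picking up, dragging and tilting interactable props such as the spoon, lighter and dropper.
; A sphere trace under the finger grabs the prop or opens TableWidget on a Pin, and releasing returns the prop.
; While held, a gated axis event moves the prop and Mouse actor to a PhysicsBody trace, easing rotation to zero.
; Holding Dotouch instead maps horizontal drag to an angle, sent through message calls.
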(event Custom|DoActor
  (bind (_locationx _locationy) (Game|Player|GetMousePosition))
  (bind _hitactor (Variables|Default|GetHitActor))
  (Utilities|IsValid _hitactor
    (:Is%20Valid
      (Utilities|FlowControl|Sequence
        (:then_0
          (Utilities|FlowControl|DoOnce false
            (:Completed
              (Variables|Default|SetStartXLoc _locationx)
              (Variables|Default|SetStartYLoc _locationy))))
        (:then_1
          (Class|InteractionInterface|DoThing(Message) _hitactor (Math|Float|Lerp 0.0 1.8e+02 (Math|Float|Clamp(Float) (/ (- _locationx (Variables|Default|GetStartXLoc)) 5e+02) -1.0)) true))))))

(event Custom|ResetDoing
  (bind (_locationx _locationy) (Game|Player|GetMousePosition))
  (Utilities|FlowControl|DoOnce false) ; enters at Reset
)

(event EventBeginPlay
  (bind _outactors (Actor|GetAllActorsOfClass "/Game/Blueprints/Main/Mouse.Mouse_C"))
  (Variables|Default|SetMouse (Utilities|Array|Get(acopy) _outactors)))

(event Input|ActionEvents|InputActionDotouch
  (params (Key :type Key%20Structure :default "None"))
  (:Pressed
    (Utilities|IsValid (Variables|Default|GetHitActor)
      (:Is%20Valid
        (Variables|Default|SetisRotating true))))
  (:Released
    (Variables|Default|SetisRotating false)
    (CallFunction|ResetDoing)))

(event Input|AxisEvents|InputAxisTouch
  (params (AxisValue :type Float%20%28single-precision%29))
  (bind _returnvalue (Game|Player|GetPlayerPawn 0))
  (bind _returnvalue_2 (Transformation|GetActorLocation _returnvalue))
  (if (Variables|Default|GetisRotating)
    (CallFunction|DoActor)
    (else
      (Utilities|FlowControl|Gate true
        (:Exit
          (Utilities|IsValid (stale Input|TouchEvents|Touch1 _output_get)
            (:Is%20Valid
              (bind _outhit (Collision|LineTraceForObjects (- _returnvalue_2 "0.000000,0.000000,10.000000") (+ (* (.WorldDirection (Game|Player|ConvertMouseLocationToWorldSpace)) 1.5e+03) _returnvalue_2) (Utilities|Array|MakeArray "ObjectTypeQuery4") false 0 "None"))
              (Transformation|SetActorLocation (Variables|Default|GetMouse) (.Location (Collision|BreakHitResult _outhit)) false false)
              (Class|InteractionInterface|Move(Message) (stale Input|TouchEvents|Touch1 _output_get) (.Location (Collision|BreakHitResult _outhit)))
              (bind _angle (Class|InteractionInterface|GetRotation(Message) (stale Input|TouchEvents|Touch1 _output_get)))
              (Class|InteractionInterface|DoThing(Message) (stale Input|TouchEvents|Touch1 _output_get) (Math|Float|Lerp _angle 0.0 0.2) false))))))))

(event Input|AxisEvents|InputAxisScroll
  (params (AxisValue :type Float%20%28single-precision%29))
  (Utilities|IsValid (Variables|Default|GetHitActor)
    (:Is%20Valid
      (Variables|Default|SetDistance (+ (Variables|Default|GetDistance) AxisValue)))))

(event Input|TouchEvents|Touch1
  (params (Key :type Key%20Structure :default "None"))
  (bind _hitresult (Class|PlayerController|GetHitResultUnderFingerbyChannel "Touch1" "TraceTypeQuery1" true))
  (bind _returnvalue (Game|Player|GetPlayerPawn 0))
  (bind _self self)
  (bind _mouse (Variables|Default|GetMouse))
  (bind (_bblockinghit _binitialoverlap _time _distance _location _impactpoint _normal _impactnormal _physmat _hitactor _hitcomponent _hitbonename _bonename _hititem _elementindex _faceindex _tracestart _traceend) (Collision|BreakHitResult _hitresult))
  (bind _returnvalue_2 (Transformation|GetActorLocation _returnvalue))
  (:Pressed
    (bind _outhit (Collision|SphereTraceByChannel _tracestart _traceend 2.0 "TraceTypeQuery1" true 0 "None"))
    (Input|SetInputModeGameOnly _self false)
    (if (.bBlockingHit (Collision|BreakHitResult _outhit))
      (if (Math|Boolean|ORBoolean (.ReturnValue (|CheckIsInter (.HitActor (Collision|BreakHitResult _outhit)) (.HitActor (Collision|BreakHitResult _outhit)) (.HitActor (Collision|BreakHitResult _outhit)) (.HitActor (Collision|BreakHitResult _outhit)))) (.ReturnValue2 (|CheckIsInter (.HitActor (Collision|BreakHitResult _outhit)) (.HitActor (Collision|BreakHitResult _outhit)) (.HitActor (Collision|BreakHitResult _outhit)) (.HitActor (Collision|BreakHitResult _outhit)))) (.ReturnValue3 (|CheckIsInter (.HitActor (Collision|BreakHitResult _outhit)) (.HitActor (Collision|BreakHitResult _outhit)) (.HitActor (Collision|BreakHitResult _outhit)) (.HitActor (Collision|BreakHitResult _outhit)))) (.ReturnValue4 (|CheckIsInter (.HitActor (Collision|BreakHitResult _outhit)) (.HitActor (Collision|BreakHitResult _outhit)) (.HitActor (Collision|BreakHitResult _outhit)) (.HitActor (Collision|BreakHitResult _outhit)))))
        (Utilities|FlowControl|Sequence
          (:then_0
            (bind _output_get (Variables|Default|SetHitActor (.HitActor (Collision|BreakHitResult _outhit))))
            (Variables|Default|SetDistance (.x (Transformation|GetActorLocation _output_get))))
          (:then_1
            (Utilities|FlowControl|Gate true) ; enters at Open
          ))
        (elif (Class|GameplayStatics|ObjectIsA (.HitActor (Collision|BreakHitResult _outhit)) "/Game/Blueprints/Main/Pin.Pin_C")
          (bind _returnvalue_3 (UserInterface|CreateWidget "/Game/Blueprints/UI/TableWidget.TableWidget_C"))
          (UserInterface|Viewport|AddtoViewport _returnvalue_3 0)))))
  (:Released
    (Input|SetInputModeGameandUI _self 0 "DoNotLock" true false)
    (Utilities|FlowControl|Sequence
      (:then_0
        (Utilities|FlowControl|Gate true) ; enters at Close
      )
      (:then_1
        (Variables|Default|SetDistance 0.0)
        (Utilities|IsValid (Variables|Default|GetHitActor)
          (:Is%20Valid
            (Variables|Default|SetInitLoc (Transformation|GetActorLocation (Variables|Default|GetHitActor)))
            (Class|InteractionInterface|Return(Message) (Variables|Default|GetHitActor))
            (Variables|Default|SetHitActor 0)
            (Transformation|SetActorLocation _mouse "0, 0, 0" false false)))))))

(fn ConstructionScript)

(fn DoThing
  (params (Angle :type Float%20%28double-precision%29) (Press :type Boolean))
  (return))

(fn GetRotation
  (return 0.0))