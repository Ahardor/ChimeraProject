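; Draggable dropper actor that holds a colored liquid compound, snaps onto interaction actors and dispenses into them while pressed.
; Sphere overlaps with tagged components drive snap and release; timers ease it into position or back to its base.
; Each tick, box traces find liquid bounds, a Cube placed by fill ratio feeds the material's fill volume, and spill state updates.
; Spilling timers drain fill, while line traces pass it to the actor below alongside Niagara particles.
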(event OnComponentBeginOverlap(Sphere)
  (params (OverlappedComponent :type Primitive%20Component%20Object%20Reference) (OtherActor :type Actor%20Object%20Reference) (OtherComp :type Primitive%20Component%20Object%20Reference) (OtherBodyIndex :type Integer) (bFromSweep :type Boolean) (SweepResult :type Hit%20Result%20Structure%20%28by%20ref%29))
  (if (not (Variables|Default|GetSnapped))
    (if (Variables|Default|GetMoving)
      (if (Utilities|Array|ContainsItem (Variables|/Script/Engine.ActorComponent|GetComponentTags OtherComp) "Detect")
        (bind _asbase_interaction_actor (Utilities|Casting|CastToBaseInteractionActor OtherActor))
        (Variables|Default|SetSnappedActor _asbase_interaction_actor)
        (Variables|Default|SetSnapped true)
        (bind _returnvalue (Utilities|Time|SetTimerbyEvent (delegate Custom|RotationSnap) 0.01 true))
        (Variables|Default|SetSpillLocTimer _returnvalue)))))

(event OnComponentEndOverlap(Sphere)
  (params (OverlappedComponent :type Primitive%20Component%20Object%20Reference) (OtherActor :type Actor%20Object%20Reference) (OtherComp :type Primitive%20Component%20Object%20Reference) (OtherBodyIndex :type Integer))
  (if (not (Variables|Default|GetSpilling))
    (if (== OtherActor (Variables|Default|GetSnappedActor))
      (if (Utilities|Array|ContainsItem (Variables|/Script/Engine.ActorComponent|GetComponentTags OtherComp) "Release")
        (if (Variables|Default|GetSnapped)
          (CallFunction|Release (Variables|Default|GetMoving)))))))

(event Custom|MoveDown
  (bind _returnvalue (Transformation|GetActorLocation))
  (bind _base (Variables|Default|GetBase))
  (bind _returnvalue_2 (Transformation|GetActorLocation _base))
  (bind _returnvalue_3 (- _returnvalue_2 "0.000000,0.000000,1.000000"))
  (bind _returnvalue_4 (Math|Vector|Lerp(Vector) _returnvalue _returnvalue_3 0.1))
  (if (Variables|Default|GetSnapped)
    (Transformation|SetWorldLocation (Variables|Default|GetSphere) _returnvalue_4 false false)
    (else
      (Transformation|SetActorLocation _returnvalue_4 false false)))
  (if (Utilities|Operators|EqualEqual (Transformation|GetActorLocation) _returnvalue_3 0.1)
    (Utilities|Time|ClearandInvalidateTimerbyHandle (stale EventReturn _returnvalue))))

(event Custom|Fulfill
  (CallFunction|AddFill (Variables|Default|GetMaxFill)))

(event Custom|RotationSnap
  (Transformation|SetActorLocation (Math|Vector|Lerp(Vector) (Transformation|GetActorLocation) (Math|Vector|MakeVector (.x (Transformation|GetWorldLocation (Variables|/Game/Blueprints/Main/BaseInteractionActor.BaseInteractionActor_C|GetSnap (stale OnComponentBeginOverlap(Sphere) _asbase_interaction_actor)))) (+ (.y (Transformation|GetWorldLocation (Variables|/Game/Blueprints/Main/BaseInteractionActor.BaseInteractionActor_C|GetSnap (stale OnComponentBeginOverlap(Sphere) _asbase_interaction_actor)))) (- (.y (Transformation|GetActorLocation)) (select (Utilities|Operators|EqualEqual :A (Variables|Default|GetSpillPoint)) (.y (Transformation|GetWorldLocation (Variables|Default|GetUpCheckPoint))) (.y (Variables|Default|GetSpillPoint))))) (.z (Transformation|GetWorldLocation (Variables|/Game/Blueprints/Main/BaseInteractionActor.BaseInteractionActor_C|GetSnap (stale OnComponentBeginOverlap(Sphere) _asbase_interaction_actor))))) 0.3) false false))

(event EventTick
  (params (DeltaSeconds :type Float%20%28single-precision%29))
  (CallFunction|CheckDown)
  (CallFunction|CheckUp)
  (CallFunction|SetMPCParams)
  (CallFunction|SetCubeHeight)
  (CallFunction|CheckSpill)
  (CallFunction|SpawnFX))

(event EventBeginPlay
  (Effects|Components|ParticleSystem|SetColorParameter (Variables|Default|GetNiagara) "ParticleColor" (Variables|Default|GetColor))
  (if (== (Variables|Default|GetFill) 0.0)
    (Rendering|SetVisibility (Variables|Default|GetStaticMesh1) false false)))

(event EventRelease
  (params (Moving :type Boolean))
  (Variables|Default|SetMoving Moving)
  (Transformation|SetWorldLocation (Variables|Default|GetSphere) (Transformation|GetWorldLocation (Variables|Default|GetScene)) false false)
  (Variables|Default|SetSnapped false)
  (Utilities|Time|ClearandInvalidateTimerbyHandle (Variables|Default|GetSpillLocTimer)))

(event EventMove
  (params (Loc :type Vector :default "0, 0, 0"))
  (bind _returnvalue (Transformation|GetActorLocation))
  (bind _returnvalue_2 (+ Loc "0.000000,0.000000,20.000000"))
  (bind _snapped (Variables|Default|GetSnapped))
  (bind _sphere (Variables|Default|GetSphere))
  (bind _returnvalue_3 (Transformation|GetWorldLocation _sphere))
  (bind _returnvalue_4 (select _snapped _returnvalue_3 _returnvalue))
  (bind _returnvalue_5 (Math|Vector|Lerp(Vector) _returnvalue_4 _returnvalue_2 0.5))
  (Variables|Default|SetMoving true)
  (if (Variables|Default|GetSnapped)
    (Transformation|SetWorldLocation (Variables|Default|GetSphere) _returnvalue_5 false false)
    (else
      (Transformation|SetActorLocation _returnvalue_5 false false))))

(event EventReturn
  (bind _returnvalue (Utilities|Time|SetTimerbyEvent (delegate Custom|MoveDown) 0.001 true))
  (bind _output_get (Variables|Default|SetMoving false))
  (CallFunction|Release _output_get))

(fn ConstructionScript
  (CallFunction|CheckDown)
  (CallFunction|CheckUp)
  (CallFunction|SetMPCParams)
  (CallFunction|SetCubeHeight)
  (CallFunction|CheckSpill)
  (CallFunction|SpawnFX))

(fn SetCubeHeight
  (bind _cube (Variables|Default|GetCube))
  (bind _indicator (Variables|Default|GetIndicator))
  (bind _returnvalue (Transformation|GetSocketLocation _indicator "Up"))
  (bind _returnvalue_2 (Transformation|GetSocketLocation _indicator "Down"))
  (Transformation|SetWorldLocation _cube (Math|Vector|MakeVector (/ (+ (.x _returnvalue) (.x _returnvalue_2)) 2.0) (/ (+ (.y _returnvalue) (.y _returnvalue_2)) 2.0) (+ (Math|Float|Lerp (Variables|Default|GetDownPoint) (Variables|Default|GetUpPoint) (/ (Variables|Default|GetFill) (Variables|Default|GetMaxFill))) (.z (.BoxExtent (Collision|GetComponentBounds _cube))))) false false))

(fn CheckSpill
  (if (!= (Variables|Default|GetFill) 0.0)
    (if (Variables|Default|GetPressed)
      (if (not (Variables|Default|GetSpilling))
        (Variables|Default|SetSpilling true)
        (bind _returnvalue (Utilities|Time|SetTimerbyFunctionName 0 "Spill" 0.01 true))
        (Variables|Default|SetSpillTimer _returnvalue)
        (bind _returnvalue_2 (Utilities|Time|SetTimerbyFunctionName 0 "CheckInteraction" 0.01 true))
        (Variables|Default|SetSpillInterTimer _returnvalue_2))
      (else
        (Utilities|Time|ClearandInvalidateTimerbyHandle (Variables|Default|GetSpillTimer) :!label _label)
        (Utilities|Time|ClearandInvalidateTimerbyHandle (Variables|Default|GetSpillInterTimer))
        (Variables|Default|SetSpilling false)
        (Variables|Default|SetSpillPoint "0, 0, 0")))
    (else
      (goto _label))))

(fn Spill
  (bind _compound (Variables|Default|GetCompound))
  (bind _niagara (Variables|Default|GetNiagara))
  (bind _spillrate (Variables|Default|GetSpillRate))
  (if (!= (Variables|Default|GetFill) 0.0)
    (Effects|Components|ParticleSystem|SetFloatParameter _niagara "SpawnRate" 1e+03)
    (Effects|Components|ParticleSystem|SetFloatParameter _niagara "SpawnRadius" 0.1)
    (bind _output_get (Variables|Default|SetSpillPoint (- (Transformation|GetWorldLocation (Variables|Default|GetStaticMesh1)) "")))
    (Transformation|SetWorldLocation (Variables|Default|GetNiagara) _output_get false false)
    (bind _output_get_2 (Variables|Default|SetFill (Math|Float|Clamp(Float) (- (Variables|Default|GetFill) _spillrate) 0.0 (Variables|Default|GetMaxFill))))
    (for (_ _array_index) _compound
      (Utilities|Struct|SetmembersinCompound (Utilities|Array|Get(acopy) _compound _array_index) (- (.Amount (Utilities|Struct|BreakCompound (Utilities|Array|Get(acopy) _compound _array_index))) (/ _spillrate (Utilities|Array|Length _compound)))))
    (if (== _output_get_2 0.0)
      (Rendering|SetVisibility (Variables|Default|GetStaticMesh1) false false))))

(fn CheckDown
  (bind _raypointdown (Variables|Default|GetRaypointDown))
  (bind _returnvalue (Transformation|GetWorldLocation _raypointdown))
  (bind _outactors (Actor|GetAllActorsOfClass "Dropper_C"))
  (LocalVariables|SetArr _outactors)
  (bind _outactors_2 (Actor|GetAllActorsOfClass "/Game/Blueprints/Main/BaseInteractionActor.BaseInteractionActor_C"))
  (bind _outactors_3 (Actor|GetAllActorsOfClass "/Game/Blueprints/Main/Spoon.Spoon_C"))
  (Utilities|Array|AppendArray (LocalVariables|GetArr) _outactors_2)
  (Utilities|Array|AppendArray (LocalVariables|GetArr) _outactors_3)
  (Utilities|Array|RemoveItem (LocalVariables|GetArr) self)
  (bind _outhit (Class|KismetSystemLibrary|BoxTraceSingleforObjects _returnvalue (+ _returnvalue "0.000000,0.000000,300.000000") "0.000000,70.000000,0.000000" "0, 0, 0" (Utilities|Array|MakeArray "ObjectTypeQuery3") true (LocalVariables|GetArr) "None" false))
  (Variables|Default|SetDownPoint (+ (.Z (Math|Vector|BreakVector (.Location (Collision|BreakHitResult _outhit)))) (Variables|Default|GetDownOffset))))

(fn CheckUp
  (bind _raypointup (Variables|Default|GetRaypointUp))
  (bind _returnvalue (Transformation|GetWorldLocation _raypointup))
  (bind _outactors (Actor|GetAllActorsOfClass "Dropper_C"))
  (LocalVariables|SetArr _outactors)
  (bind _outactors_2 (Actor|GetAllActorsOfClass "/Game/Blueprints/Main/BaseInteractionActor.BaseInteractionActor_C"))
  (bind _outactors_3 (Actor|GetAllActorsOfClass "/Game/Blueprints/Main/Spoon.Spoon_C"))
  (Utilities|Array|AppendArray (LocalVariables|GetArr) _outactors_2)
  (Utilities|Array|AppendArray (LocalVariables|GetArr) _outactors_3)
  (Utilities|Array|RemoveItem (LocalVariables|GetArr) self)
  (bind _outhit (Class|KismetSystemLibrary|BoxTraceSingleforObjects _returnvalue (+ _returnvalue "0.000000,0.000000,-100.000000") "0.000000,70.000000,0.000000" "0, 0, 0" (Utilities|Array|MakeArray "ObjectTypeQuery3") true (LocalVariables|GetArr) "None" false))
  (Variables|Default|SetUpPoint (.Z (Math|Vector|BreakVector (.Location (Collision|BreakHitResult _outhit))))))

(fn SetMPCParams
  (bind _cube (Variables|Default|GetCube))
  (bind _staticmesh1 (Variables|Default|GetStaticMesh1))
  (bind _returnvalue (Transformation|GetWorldTransform _cube))
  (bind _returnvalue_2 (Rendering|Material|CreateDynamicMaterialInstance _staticmesh1 0 (Rendering|Material|GetMaterial _staticmesh1 0) "None" :!class /Script/Engine.PrimitiveComponent))
  (Rendering|Material|SetVectorParameterValue _returnvalue_2 "Location" (Math|Conversions|ToLinearColor(Vector) (.location _returnvalue)) :!class /Script/Engine.MaterialInstanceDynamic)
  (Rendering|Material|SetVectorParameterValue _returnvalue_2 "Scale" (Math|Conversions|ToLinearColor(Vector) (.scale _returnvalue)) :!class /Script/Engine.MaterialInstanceDynamic)
  (Rendering|Material|SetVectorParameterValue _returnvalue_2 "Color" (Variables|Default|GetColor) :!class /Script/Engine.MaterialInstanceDynamic))

(fn SpawnFX
  (bind _niagara (Variables|Default|GetNiagara))
  (if (!= (Variables|Default|GetFill) 0.0)
    (if (Variables|Default|GetPressed)
      (if (not (Variables|Default|GetSpawnedParticle))
        (Variables|Default|SetSpawnedParticle true)
        (Components|Activation|Activate _niagara true))
      (else
        (if (Variables|Default|GetSpawnedParticle) :!label _label
          (Variables|Default|SetSpawnedParticle false)
          (Components|Activation|Deactivate _niagara))))
    (else
      (goto _label))))

(fn CheckInteraction
  (bind _spillpoint (Variables|Default|GetSpillPoint))
  (if (Variables|Default|GetSpilling)
    (bind _outhits (Collision|MultiLineTraceByChannel _spillpoint (- _spillpoint "0.000000,0.000000,200.000000") "TraceTypeQuery1" true 0 "None"))
    (bind _array_element (Utilities|Array|ForEachLoopwithBreak _outhits :!label _label)
      (:LoopBody
        (bind _asbase_interaction_actor (Utilities|Casting|CastToBaseInteractionActor (.HitActor (Collision|BreakHitResult _array_element))))
        (Default|AddFill _asbase_interaction_actor (Variables|Default|GetSpillRate) (Variables|Default|GetCompound))
        (goto _label Break)))))

(fn AddFill
  (params (Amount :type Float%20%28double-precision%29))
  (if (== (Variables|Default|GetFill) 0.0)
    (Rendering|SetVisibility (Variables|Default|GetStaticMesh1) true false)
    (Utilities|Struct|SetmembersinCompound (Utilities|Array|Get(acopy) (Variables|Default|GetCompound)) (Math|Float|Clamp(Float) (+ (Variables|Default|GetFill) Amount) 0.0 (Variables|Default|GetMaxFill)))
    (Effects|Components|ParticleSystem|SetColorParameter (Variables|Default|GetNiagara) "ParticleColor" (Variables|Default|GetColor))
    (bind _output_get (Variables|Default|SetFill (Math|Float|Clamp(Float) (+ (Variables|Default|GetFill) Amount) 0.0 (Variables|Default|GetMaxFill))))
    (if (< _output_get (Variables|Default|GetMaxFill))
      (CallFunction|ComputeColor))))

(fn ComputeColor
  (for _array_element (Variables|Default|GetCompound)
    (LocalVariables|SetColorLocal (Math|Color|Lerp(LinearColor) (LocalVariables|GetColorLocal) (.Color (Utilities|Struct|BreakCompound _array_element)) (/ (.Amount (Utilities|Struct|BreakCompound _array_element)) (Variables|Default|GetFill)))))
  (Variables|Default|SetColor (LocalVariables|GetColorLocal)))

(fn DoThing
  (params (Angle :type Float%20%28double-precision%29) (Press :type Boolean))
  (Variables|Default|SetPressed Press)
  (return))

(fn GetRotation
  (return (Variables|Default|GetAngle)))