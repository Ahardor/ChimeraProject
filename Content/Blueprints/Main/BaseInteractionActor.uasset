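; Base movable liquid container that pours chemical compounds into other containers and snaps to them or EtanolFire while dragged.
; Each tick, box traces find the tilted vessel's vertical bounds, placing a Cube at fill height to drive the liquid material.
; When that Cube stops overlapping both marker cubes, timers drain Fill, drive Niagara and trace downward for a receiving container.
; Receivers merge compounds, recompute blended color and play fill audio.
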(event OnComponentBeginOverlap(Sphere)
  (params (OverlappedComponent :type Primitive%20Component%20Object%20Reference) (OtherActor :type Actor%20Object%20Reference) (OtherComp :type Primitive%20Component%20Object%20Reference) (OtherBodyIndex :type Integer) (bFromSweep :type Boolean) (SweepResult :type Hit%20Result%20Structure%20%28by%20ref%29))
  (if (not (Variables|Default|GetSnapped))
    (if (Variables|Default|GetMoving)
      (if (Utilities|Array|ContainsItem (Variables|/Script/Engine.ActorComponent|GetComponentTags OtherComp) "Detect")
        (bind _asbase_interaction_actor (Utilities|Casting|CastToBaseInteractionActor OtherActor)
          (:then
            (Variables|Default|SetSnapEtanol false)
            (Variables|Default|SetSnappedActor _asbase_interaction_actor))
          (:CastFailed
            (bind _asetanol_fire (Utilities|Casting|CastToEtanolFire OtherActor))
            (Variables|Default|SetSnapEtanol true)
            (Variables|Default|SetSnappedActor _asetanol_fire)))
        (Variables|Default|SetSnapped true)
        (bind _returnvalue (Utilities|Time|SetTimerbyEvent (delegate Custom|RotationSnap) 0.01 true))
        (Variables|Default|SetSpillLocTimer _returnvalue)))))

(event OnComponentEndOverlap(Sphere)
  (params (OverlappedComponent :type Primitive%20Component%20Object%20Reference) (OtherActor :type Actor%20Object%20Reference) (OtherComp :type Primitive%20Component%20Object%20Reference) (OtherBodyIndex :type Integer))
  (if (not (Variables|Default|GetSpilling))
    (if (== OtherActor (Variables|Default|GetSnappedActor))
      (if (Utilities|Array|ContainsItem (Variables|/Script/Engine.ActorComponent|GetComponentTags OtherComp) "Release")
        (if (Variables|Default|GetSnapped)
          (Default|Release self (Variables|Default|GetMoving)))))))

(event Custom|MoveDown
  (bind _returnvalue (Transformation|GetActorLocation))
  (bind _initplaceloc (Variables|Default|GetInitPlaceLoc))
  (bind _placeloc (Variables|Default|GetPlaceLoc))
  (bind _returnvalue_2 (Utilities|Operators|NotEqual(!=) :A _placeloc :ErrorTolerance 0.1))
  (bind _returnvalue_3 (select _returnvalue_2 _placeloc _initplaceloc))
  (bind _returnvalue_4 (Math|Vector|Lerp(Vector) _returnvalue _returnvalue_3 0.05))
  (CallFunction|DoThing 0.0 false)
  (if (Variables|Default|GetSnapped)
    (Transformation|SetWorldLocation (Variables|Default|GetSphere) _returnvalue_4 false false)
    (else
      (Transformation|SetActorLocation _returnvalue_4 false false)))
  (if (Utilities|Operators|EqualEqual (Transformation|GetActorLocation) _returnvalue_3 0.1)
    (Utilities|Time|ClearandInvalidateTimerbyHandle (stale EventReturn _returnvalue))))

(event Custom|PlayAudio
  (bind _audio (Variables|Default|GetAudio))
  (Components|Activation|Activate _audio false)
  (Utilities|FlowControl|Sequence
    (:then_0
      (Utilities|FlowControl|DoOnce false
        (:Completed
          (Audio|Components|Audio|Play _audio (* (Variables|/Script/Engine.SoundBase|GetDuration (Variables|/Script/Engine.AudioComponent|GetSound _audio)) (/ (Variables|Default|GetFill) (Variables|Default|GetMaxFill)) 0.5)))))
    (:then_1
      (Utilities|Time|SetTimerbyEvent (delegate Custom|DeactivateAudio) 0.2))))

(event Custom|RotationSnap
  (Transformation|SetActorLocation (Math|Vector|Lerp(Vector) (Transformation|GetActorLocation) (Math|Vector|MakeVector (.x (Transformation|GetWorldLocation (select (Variables|Default|GetSnapEtanol) (Variables|/Game/Blueprints/Main/EtanolFire.EtanolFire_C|GetSnap (stale OnComponentBeginOverlap(Sphere) _asetanol_fire)) (Variables|BaseInteractionActor_C|GetSnap (stale OnComponentBeginOverlap(Sphere) _asbase_interaction_actor))))) (+ (.y (Transformation|GetWorldLocation (select (Variables|Default|GetSnapEtanol) (Variables|/Game/Blueprints/Main/EtanolFire.EtanolFire_C|GetSnap (stale OnComponentBeginOverlap(Sphere) _asetanol_fire)) (Variables|BaseInteractionActor_C|GetSnap (stale OnComponentBeginOverlap(Sphere) _asbase_interaction_actor))))) (- (.y (Transformation|GetActorLocation)) (select (Utilities|Operators|EqualEqual :A (Variables|Default|GetSpillPoint)) (.y (Transformation|GetWorldLocation (Variables|Default|GetUpCheckPoint))) (.y (Variables|Default|GetSpillPoint))))) (.z (Transformation|GetWorldLocation (select (Variables|Default|GetSnapEtanol) (Variables|/Game/Blueprints/Main/EtanolFire.EtanolFire_C|GetSnap (stale OnComponentBeginOverlap(Sphere) _asetanol_fire)) (Variables|BaseInteractionActor_C|GetSnap (stale OnComponentBeginOverlap(Sphere) _asbase_interaction_actor)))))) 0.3) false false))

(event Custom|DeactivateAudio
  (bind _audio (Variables|Default|GetAudio))
  (Components|Activation|Deactivate _audio)
  (Utilities|FlowControl|DoOnce false) ; enters at Reset
)

(event EventTick
  (params (DeltaSeconds :type Float%20%28single-precision%29))
  (CallFunction|CheckDown)
  (CallFunction|CheckUp)
  (CallFunction|SetMPCParams)
  (CallFunction|SetCubeHeight)
  (CallFunction|CheckSpill)
  (CallFunction|SpawnFX)
  (CallFunction|GetPlacePoint)
  (CallFunction|SetText))

(event EventBeginPlay
  (Effects|Components|ParticleSystem|SetColorParameter (Variables|Default|GetNiagara) "ParticleColor" (Variables|Default|GetColor))
  (if (== (Variables|Default|GetFill) 0.0)
    (Rendering|SetVisibility (Variables|Default|GetStaticMesh1) false false))
  (Variables|Default|SetInitPlaceLoc (Transformation|GetActorLocation))
  (Variables|Default|SetParticleInit (Variables|Default|GetStaticMesh))
  (Class|AudioComponent|SetPaused (Variables|Default|GetAudio1) true))

(event EventRelease
  (params (Moving :type Boolean))
  (Variables|Default|SetMoving Moving)
  (Transformation|SetWorldLocation (Variables|Default|GetSphere) (Transformation|GetWorldLocation (Variables|Default|GetScene)) false false)
  (Variables|Default|SetSnapped false)
  (Utilities|Time|ClearandInvalidateTimerbyHandle (Variables|Default|GetSpillLocTimer)))

(event EventMove
  (params (Loc :type Vector :default "0, 0, 0"))
  (bind _returnvalue (Transformation|GetActorLocation))
  (bind _returnvalue_2 (+ Loc "0.000000,0.000000,20.000000"))
  (bind _sphere (Variables|Default|GetSphere))
  (bind _snapped (Variables|Default|GetSnapped))
  (bind _returnvalue_3 (Transformation|GetWorldLocation _sphere))
  (bind _returnvalue_4 (select _snapped _returnvalue_3 _returnvalue))
  (bind _returnvalue_5 (Math|Vector|Lerp(Vector) _returnvalue_4 _returnvalue_2 0.5))
  (Variables|Default|SetMoving true)
  (if (Variables|Default|GetSnapped)
    (Transformation|SetWorldLocation (Variables|Default|GetSphere) _returnvalue_5 false false)
    (else
      (Transformation|SetActorLocation _returnvalue_5 false false))))

(event EventReturn
  (bind _returnvalue (Utilities|Time|SetTimerbyEvent (delegate Custom|MoveDown) 0.001 true))
  (bind _output_get (Variables|Default|SetMoving false))
  (CallFunction|Release _output_get))

(fn ConstructionScript
  (CallFunction|CheckDown)
  (CallFunction|CheckUp)
  (CallFunction|SetMPCParams)
  (CallFunction|SetCubeHeight)
  (CallFunction|CheckSpill)
  (CallFunction|SpawnFX)
  (CallFunction|SetText))

(fn SetCubeHeight
  (bind _staticmesh (Variables|Default|GetStaticMesh))
  (bind _cube (Variables|Default|GetCube))
  (bind _returnvalue (Transformation|GetSocketLocation _staticmesh "Up"))
  (bind _returnvalue_2 (Transformation|GetSocketLocation _staticmesh "Down"))
  (Transformation|SetWorldLocation _cube (Math|Vector|MakeVector (/ (+ (.x _returnvalue) (.x _returnvalue_2)) 2.0) (/ (+ (.y _returnvalue) (.y _returnvalue_2)) 2.0) (+ (Math|Float|Lerp (Variables|Default|GetDownPoint) (Variables|Default|GetUpPoint) (/ (Variables|Default|GetFill) (Variables|Default|GetMaxFill))) (.z (.BoxExtent (Collision|GetComponentBounds _cube))))) false false))

(fn CheckSpill
  (bind _cube (Variables|Default|GetCube))
  (bind _outoverlappingcomponents (Class|PrimitiveComponent|GetOverlappingComponents _cube))
  (if (!= (Variables|Default|GetFill) 0.0)
    (if (not (and (Utilities|Array|ContainsItem _outoverlappingcomponents (Variables|Default|GetCube1)) (Utilities|Array|ContainsItem _outoverlappingcomponents (Variables|Default|GetCube2))))
      (if (not (Variables|Default|GetSpilling))
        (Variables|Default|SetSpilling true)
        (bind _returnvalue (Utilities|Time|SetTimerbyFunctionName 0 "Spill" 0.01 true))
        (Variables|Default|SetSpillTimer _returnvalue)
        (bind _returnvalue_2 (Utilities|Time|SetTimerbyFunctionName 0 "CheckInteraction" 0.01 true))
        (Variables|Default|SetSpillInterTimer _returnvalue_2))
      (else
        (Utilities|Time|ClearandInvalidateTimerbyHandle (Variables|Default|GetSpillTimer) :!label _label)
        (Utilities|Time|ClearandInvalidateTimerbyHandle (Variables|Default|GetSpillInterTimer))
        (Variables|Default|SetSpilling false)
        (Variables|Default|SetSpillPoint "0, 0, 0")
        (Class|AudioComponent|SetPaused (Variables|Default|GetAudio1) true)))
    (else
      (Utilities|Array|Clear (Variables|Default|GetCompound))
      (goto _label))))

(fn Spill
  (bind _compound (Variables|Default|GetCompound))
  (bind _minspillrate (Variables|Default|GetMinSpillRate))
  (bind _maxspillrate (Variables|Default|GetMaxSpillRate))
  (bind _angle (Variables|Default|GetAngle))
  (bind _niagara (Variables|Default|GetNiagara))
  (bind _returnvalue (Math|Float|Absolute(Float) _angle))
  (bind _returnvalue_2 (/ _returnvalue 9e+01))
  (bind _returnvalue_3 (Math|Float|Lerp _minspillrate _maxspillrate _returnvalue_2))
  (if (!= (Variables|Default|GetFill) 0.0)
    (Effects|Components|ParticleSystem|SetFloatParameter _niagara "SpawnRate" (Math|Float|Lerp 1e+01 (* (Variables|Default|GetMaxSpillRadius) 3e+03) _returnvalue_2))
    (Effects|Components|ParticleSystem|SetFloatParameter _niagara "SpawnRadius" (Math|Float|Lerp 0.2 (Variables|Default|GetMaxSpillRadius) _returnvalue_2))
    (bind _output_get (Variables|Default|SetSpillPoint (Math|Vector|Lerp(Vector) (Transformation|GetWorldLocation (Variables|Default|GetParticleInit)) (- (/ (+ (Transformation|GetWorldLocation (Variables|Default|GetCube1)) (Transformation|GetWorldLocation (Variables|Default|GetCube2))) 2.0) (Variables|Default|GetParticleOffset)) (Math|Float|Clamp(Float) (/ (- _returnvalue 9e+01) 9e+01)))))
    (Transformation|SetWorldLocation (Variables|Default|GetNiagara) _output_get false false)
    (bind _output_get_2 (Variables|Default|SetSpillRate _returnvalue_3))
    (bind _output_get_3 (Variables|Default|SetFill (Math|Float|Clamp(Float) (- (Variables|Default|GetFill) _returnvalue_3) 0.0 (Variables|Default|GetMaxFill))))
    (for (_ _array_index) _compound
      (Utilities|Struct|SetmembersinCompound (Utilities|Array|Get(acopy) _compound _array_index) (- (.Amount (Utilities|Struct|BreakCompound (Utilities|Array|Get(acopy) _compound _array_index))) (* (/ (.Amount (Utilities|Struct|BreakCompound (Utilities|Array|Get(acopy) _compound _array_index))) _output_get_3) _output_get_2))))
    (if (== _output_get_3 0.0)
      (Rendering|SetVisibility (Variables|Default|GetStaticMesh1) false false))))

(fn CheckDown
  (bind _raypointdown (Variables|Default|GetRaypointDown))
  (bind _returnvalue (Transformation|GetWorldLocation _raypointdown))
  (bind _outactors (Actor|GetAllActorsOfClass "/Game/Blueprints/Main/Dropper.Dropper_C"))
  (LocalVariables|SetArr _outactors)
  (bind _outactors_2 (Actor|GetAllActorsOfClass "BaseInteractionActor_C"))
  (bind _outactors_3 (Actor|GetAllActorsOfClass "/Game/Blueprints/Main/Spoon.Spoon_C"))
  (Utilities|Array|AppendArray (LocalVariables|GetArr) _outactors_2)
  (Utilities|Array|AppendArray (LocalVariables|GetArr) _outactors_3)
  (Utilities|Array|RemoveItem (LocalVariables|GetArr) self)
  (bind _outhit (Class|KismetSystemLibrary|BoxTraceSingleforObjects _returnvalue (+ _returnvalue "0.000000,0.000000,300.000000") "0.000000,70.000000,0.000000" "0, 0, 0" (Utilities|Array|MakeArray "ObjectTypeQuery3") true (LocalVariables|GetArr) "None" false))
  (Variables|Default|SetDownPoint (+ (.Z (Math|Vector|BreakVector (.Location (Collision|BreakHitResult _outhit)))) (Variables|Default|GetDownOffset))))

(fn CheckUp
  (bind _raypointup (Variables|Default|GetRaypointUp))
  (bind _returnvalue (Transformation|GetWorldLocation _raypointup))
  (bind _outactors (Actor|GetAllActorsOfClass "/Game/Blueprints/Main/Dropper.Dropper_C"))
  (LocalVariables|SetArr _outactors)
  (bind _outactors_2 (Actor|GetAllActorsOfClass "BaseInteractionActor_C"))
  (bind _outactors_3 (Actor|GetAllActorsOfClass "/Game/Blueprints/Main/Spoon.Spoon_C"))
  (Utilities|Array|AppendArray (LocalVariables|GetArr) _outactors_2)
  (Utilities|Array|AppendArray (LocalVariables|GetArr) _outactors_3)
  (Utilities|Array|RemoveItem (LocalVariables|GetArr) self)
  (bind _outhit (Class|KismetSystemLibrary|BoxTraceSingleforObjects _returnvalue (+ _returnvalue "0.000000,0.000000,-100.000000") "0.000000,70.000000,0.000000" "0, 0, 0" (Utilities|Array|MakeArray "ObjectTypeQuery3") true (LocalVariables|GetArr) "None" false))
  (Variables|Default|SetUpPoint (.Z (Math|Vector|BreakVector (.Location (Collision|BreakHitResult _outhit))))))

(fn SetMPCParams
  (bind _cube (Variables|Default|GetCube))
  (bind _staticmesh1 (Variables|Default|GetStaticMesh1))
  (bind _returnvalue (Transformation|GetWorldTransform _cube))
  (bind _returnvalue_2 (Rendering|Material|CreateDynamicMaterialInstance _staticmesh1 0 (Rendering|Material|GetMaterial _staticmesh1 0) "None" :!class /Script/Engine.PrimitiveComponent))
  (Rendering|Material|SetVectorParameterValue _returnvalue_2 "Location" (Math|Conversions|ToLinearColor(Vector) (.location _returnvalue)) :!class /Script/Engine.MaterialInstanceDynamic)
  (Rendering|Material|SetVectorParameterValue _returnvalue_2 "Scale" (Math|Conversions|ToLinearColor(Vector) (.scale _returnvalue)) :!class /Script/Engine.MaterialInstanceDynamic)
  (Rendering|Material|SetVectorParameterValue _returnvalue_2 "Color" (Variables|Default|GetColor) :!class /Script/Engine.MaterialInstanceDynamic))

(fn SpawnFX
  (bind _cube (Variables|Default|GetCube))
  (bind _cube1 (Variables|Default|GetCube1))
  (bind _cube2 (Variables|Default|GetCube2))
  (bind _niagara (Variables|Default|GetNiagara))
  (bind _outoverlappingcomponents (Class|PrimitiveComponent|GetOverlappingComponents _cube))
  (bind _returnvalue (Utilities|Array|ContainsItem _outoverlappingcomponents _cube1))
  (if (!= (Variables|Default|GetFill) 0.0)
    (if (not (and _returnvalue (Utilities|Array|ContainsItem _outoverlappingcomponents _cube2)))
      (if (not (Variables|Default|GetSpawnedParticle))
        (Variables|Default|SetSpawnedParticle true)
        (Variables|Default|SetParticleInit (select _returnvalue _cube2 _cube1))
        (Components|Activation|Activate _niagara true))
      (else
        (if (Variables|Default|GetSpawnedParticle) :!label _label
          (Variables|Default|SetSpawnedParticle false)
          (Components|Activation|Deactivate _niagara))))
    (else
      (goto _label))))

(fn CheckInteraction
  (bind _spillpoint (Variables|Default|GetSpillPoint))
  (if (Variables|Default|GetSpilling)
    (bind _outhits (Collision|MultiLineTraceByChannel _spillpoint (- _spillpoint "0.000000,0.000000,200.000000") "TraceTypeQuery1" true 0 "None"))
    (bind _array_element (Utilities|Array|ForEachLoopwithBreak _outhits :!label _label)
      (:LoopBody
        (bind _asbase_interaction_actor (Utilities|Casting|CastToBaseInteractionActor (.HitActor (Collision|BreakHitResult _array_element)))
          (:then
            (CallFunction|AddFill _asbase_interaction_actor (Variables|Default|GetSpillRate) (Variables|Default|GetCompound))
            (goto _label Break))
          (:CastFailed
            _)))
      (:Completed
        _))
    (Class|AudioComponent|SetPaused (Variables|Default|GetAudio1) false)
    (else
      (Class|AudioComponent|SetPaused (Variables|Default|GetAudio1) true))))

(fn AddFill
  (params (Amount :type Float%20%28double-precision%29) (Comp :type Array%20of%20Compound%20Structures))
  (bind _compound (Variables|Default|GetCompound))
  (for _array_element Comp
    (LocalVariables|SetIncomeAll (+ (LocalVariables|GetIncomeAll) (.amount _array_element))))
  (for _array_element_2 Comp
    (if (== (Variables|Default|GetFill) 0.0)
      (Rendering|SetVisibility (Variables|Default|GetStaticMesh1) true false))
    (if (.Find (CallFunction|FindCompoundbyName _compound (.Name (Utilities|Struct|BreakCompound _array_element_2))))
      _
      (else
        (Utilities|Array|Add _compound (Utilities|Struct|MakeCompound (.Name (Utilities|Struct|BreakCompound _array_element_2)) (.Color (Utilities|Struct|BreakCompound _array_element_2)) 0.0))))
    (Utilities|Struct|SetmembersinCompound (Utilities|Array|Get(acopy) _compound (.Item (CallFunction|FindCompoundbyName _compound (.Name (Utilities|Struct|BreakCompound _array_element_2))))) (select (.Find (CallFunction|FindCompoundbyName _compound (.Name (Utilities|Struct|BreakCompound _array_element_2)))) (Math|Color|Lerp(LinearColor) (.Color (Utilities|Struct|BreakCompound _array_element_2)) (.Color (Utilities|Struct|BreakCompound (Utilities|Array|Get(acopy) _compound (.Item (CallFunction|FindCompoundbyName _compound (.Name (Utilities|Struct|BreakCompound _array_element_2))))))) (/ (* Amount (/ (.Amount (Utilities|Struct|BreakCompound _array_element_2)) (LocalVariables|GetIncomeAll))) (+ (.Amount (Utilities|Struct|BreakCompound (Utilities|Array|Get(acopy) _compound (.Item (CallFunction|FindCompoundbyName _compound (.Name (Utilities|Struct|BreakCompound _array_element_2))))))) (* Amount (/ (.Amount (Utilities|Struct|BreakCompound _array_element_2)) (LocalVariables|GetIncomeAll)))))) (.Color (Utilities|Struct|BreakCompound _array_element_2))) (Math|Float|SelectFloat (+ (.Amount (Utilities|Struct|BreakCompound (Utilities|Array|Get(acopy) _compound (.Item (CallFunction|FindCompoundbyName _compound (.Name (Utilities|Struct|BreakCompound _array_element_2))))))) (* Amount (/ (.Amount (Utilities|Struct|BreakCompound _array_element_2)) (LocalVariables|GetIncomeAll)))) (* Amount (/ (.Amount (Utilities|Struct|BreakCompound _array_element_2)) (LocalVariables|GetIncomeAll))) (.Find (CallFunction|FindCompoundbyName _compound (.Name (Utilities|Struct|BreakCompound _array_element_2)))))))
  (Effects|Components|ParticleSystem|SetColorParameter (Variables|Default|GetNiagara) "ParticleColor" (Variables|Default|GetColor))
  (bind _output_get (Variables|Default|SetFill (Math|Float|Clamp(Float) (+ (Variables|Default|GetFill) Amount) 0.0 (Variables|Default|GetMaxFill))))
  (if (< _output_get (Variables|Default|GetMaxFill))
    (CallFunction|ComputeColor)
    (CallFunction|PlayAudio)))

(fn ComputeColor
  (for _array_element (Variables|Default|GetCompound)
    (LocalVariables|SetColorLocal (Math|Color|Lerp(LinearColor) (LocalVariables|GetColorLocal) (.Color (Utilities|Struct|BreakCompound _array_element)) (/ (.Amount (Utilities|Struct|BreakCompound _array_element)) (Variables|Default|GetFill)))))
  (Variables|Default|SetColor (LocalVariables|GetColorLocal)))

(fn GetPlacePoint
  (bind _returnvalue (Transformation|GetActorLocation))
  (if (Variables|Default|GetMoving)
    (bind _outhit (Class|KismetSystemLibrary|LineTraceSinglebyProfile _returnvalue (+ _returnvalue (* (Transformation|GetActorUpVector) -2e+02)) "PhysicsBody" false 0 "None" true))
    (if (.bBlockingHit (Collision|BreakHitResult _outhit))
      (Variables|Default|SetPlaceLoc (.Location (Collision|BreakHitResult _outhit)))
      (else
        (Variables|Default|SetPlaceLoc "0, 0, 0")))))

(fn SetText
  (Rendering|Components|TextRender|SetText (Variables|Default|GetTextRender) (Utilities|Text|ToText(String) (Variables|Default|GetText))))

(fn DoThing
  (params (Angle :type Float%20%28double-precision%29) (Press :type Boolean))
  (Variables|Default|SetAngle Angle)
  (Transformation|SetRelativeRotation (Variables|Default|GetStaticMesh) (Math|Rotator|MakeRotator Angle 0.0 0.0) false false)
  (return))

(fn GetRotation
  (return (Variables|Default|GetAngle)))