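; Danger flask actor for Level 1 that shows its Element name on a text render and acts as a fill point for the Dropper.
; The label is set in the construction script and again at BeginPlay.
; When a Dropper enters the Sphere, the flask calls Fulfill on it and hides the Cap.
; When the Dropper leaves, the Cap becomes visible again.
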(event OnComponentBeginOverlap(Sphere)
  (params (OverlappedComponent :type Primitive%20Component%20Object%20Reference) (OtherActor :type Actor%20Object%20Reference) (OtherComp :type Primitive%20Component%20Object%20Reference) (OtherBodyIndex :type Integer) (bFromSweep :type Boolean) (SweepResult :type Hit%20Result%20Structure%20%28by%20ref%29))
  (bind _asdropper (Utilities|Casting|CastToDropper OtherActor))
  (Default|Fulfill _asdropper)
  (Rendering|SetVisibility (Variables|Default|GetCap) false false))

(event OnComponentEndOverlap(Sphere)
  (params (OverlappedComponent :type Primitive%20Component%20Object%20Reference) (OtherActor :type Actor%20Object%20Reference) (OtherComp :type Primitive%20Component%20Object%20Reference) (OtherBodyIndex :type Integer))
  (Utilities|Casting|CastToDropper OtherActor)
  (Rendering|SetVisibility (Variables|Default|GetCap) true false))

(event EventBeginPlay
  (|CallParentFunction)
  (Rendering|Components|TextRender|SetText (Variables|Default|GetTextRender) (Variables|Default|GetElement)))

(event Collision|EventActorBeginOverlap
  (params (OtherActor :type Actor%20Object%20Reference))
  (|CallParentFunction OtherActor) ; This node is disabled and will not be called.\nDrag off pins to build functionality.
)

(event EventTick
  (params (DeltaSeconds :type Float%20%28single-precision%29))
  (|CallParentFunction DeltaSeconds) ; This node is disabled and will not be called.\nDrag off pins to build functionality.
)

(fn ConstructionScript
  (|CallParentFunction)
  (Rendering|Components|TextRender|SetText (Variables|Default|GetTextRender) (Variables|Default|GetElement)))