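; Draggable lighter for Level 2 that tilts when pressed and starts the Volcano Bucket when its trigger sphere overlaps one.
; Move lerps it toward a target; touching a Detect component while moving starts a looping timer that eases it onto that actor's Snap point.
; While snapped, only the detection sphere follows input, so leaving a Release component unsnaps it.
; Return releases it and eases it back to its Base on a timer.
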(event OnComponentBeginOverlap(Sphere)
  (params (OverlappedComponent :type Primitive%20Component%20Object%20Reference) (OtherActor :type Actor%20Object%20Reference) (OtherComp :type Primitive%20Component%20Object%20Reference) (OtherBodyIndex :type Integer) (bFromSweep :type Boolean) (SweepResult :type Hit%20Result%20Structure%20%28by%20ref%29))
  (if (not (Variables|Default|GetSnapped))
    (if (Variables|Default|GetMoving)
      (if (Utilities|Array|ContainsItem (Variables|/Script/Engine.ActorComponent|GetComponentTags OtherComp) "Detect")
        (bind _asbase_interaction_actor (Utilities|Casting|CastToBaseInteractionActor OtherActor))
        (Variables|Default|SetSnappedActor _asbase_interaction_actor)
        (Variables|Default|SetSnapped true)
        (bind _returnvalue (Utilities|Time|SetTimerbyEvent (delegate Custom|RotationSnap) 0.01 true))
        (Variables|Default|SetSpillLocTimer _returnvalue)))))

(event OnComponentEndOverlap(Sphere)
  (params (OverlappedComponent :type Primitive%20Component%20Object%20Reference) (OtherActor :type Actor%20Object%20Reference) (OtherComp :type Primitive%20Component%20Object%20Reference) (OtherBodyIndex :type Integer))
  (if (not (Variables|Default|GetSpilling))
    (if (== OtherActor (Variables|Default|GetSnappedActor))
      (if (Utilities|Array|ContainsItem (Variables|/Script/Engine.ActorComponent|GetComponentTags OtherComp) "Release")
        (if (Variables|Default|GetSnapped)
          (CallFunction|Release (Variables|Default|GetMoving)))))))

(event OnComponentBeginOverlap(Sphere1)
  (params (OverlappedComponent :type Primitive%20Component%20Object%20Reference) (OtherActor :type Actor%20Object%20Reference) (OtherComp :type Primitive%20Component%20Object%20Reference) (OtherBodyIndex :type Integer) (bFromSweep :type Boolean) (SweepResult :type Hit%20Result%20Structure%20%28by%20ref%29))
  (bind _as2_volcano_bucket (Utilities|Casting|CastTo2_Volcano_Bucket OtherActor))
  (Default|Start _as2_volcano_bucket))

(event Custom|MoveDown
  (bind _returnvalue (Transformation|GetActorLocation))
  (bind _lighter (Variables|Default|GetLighter))
  (bind _base (Variables|Default|GetBase))
  (bind _returnvalue_2 (Transformation|GetActorLocation _base))
  (bind _returnvalue_3 (- _returnvalue_2 "0.000000,0.000000,1.000000"))
  (bind _returnvalue_4 (Math|Vector|Lerp(Vector) _returnvalue _returnvalue_3 0.1))
  (Transformation|SetRelativeRotation _lighter (Math|Rotator|Lerp(Rotator) (Variables|/Script/Engine.SceneComponent|GetRelativeRotation _lighter) "0, 0, 0" 0.2 true) false false)
  (if (Variables|Default|GetSnapped)
    (Transformation|SetWorldLocation (Variables|Default|GetSphere) _returnvalue_4 false false)
    (else
      (Transformation|SetActorLocation _returnvalue_4 false false)))
  (if (Utilities|Operators|EqualEqual (Transformation|GetActorLocation) _returnvalue_3 0.1)
    (Utilities|Time|ClearandInvalidateTimerbyHandle (stale EventReturn _returnvalue))))

(event Custom|RotationSnap
  (Transformation|SetActorLocation (Math|Vector|Lerp(Vector) (Transformation|GetActorLocation) (Math|Vector|MakeVector (.x (Transformation|GetWorldLocation (Variables|/Game/Blueprints/Main/BaseInteractionActor.BaseInteractionActor_C|GetSnap (stale OnComponentBeginOverlap(Sphere) _asbase_interaction_actor)))) (+ (.y (Transformation|GetWorldLocation (Variables|/Game/Blueprints/Main/BaseInteractionActor.BaseInteractionActor_C|GetSnap (stale OnComponentBeginOverlap(Sphere) _asbase_interaction_actor)))) (- (.y (Transformation|GetActorLocation)) (select (Utilities|Operators|EqualEqual :A (Variables|Default|GetSpillPoint)) (.y (Transformation|GetWorldLocation (Variables|Default|GetUpCheckPoint))) (.y (Variables|Default|GetSpillPoint))))) (.z (Transformation|GetWorldLocation (Variables|/Game/Blueprints/Main/BaseInteractionActor.BaseInteractionActor_C|GetSnap (stale OnComponentBeginOverlap(Sphere) _asbase_interaction_actor))))) 0.3) false false))

(event EventRelease
  (params (Moving :type Boolean))
  (Variables|Default|SetMoving Moving)
  (Transformation|SetWorldLocation (Variables|Default|GetSphere) (Transformation|GetWorldLocation (Variables|Default|GetScene)) false false)
  (Variables|Default|SetSnapped false)
  (Utilities|Time|ClearandInvalidateTimerbyHandle (Variables|Default|GetSpillLocTimer)))

(event EventMove
  (params (Loc :type Vector :default "0, 0, 0"))
  (bind _returnvalue (Transformation|GetActorLocation))
  (bind _returnvalue_2 (+ Loc "0.000000,0.000000,20.000000"))
  (bind _snapped (Variables|Default|GetSnapped))
  (bind _sphere (Variables|Default|GetSphere))
  (bind _returnvalue_3 (Transformation|GetWorldLocation _sphere))
  (bind _returnvalue_4 (select _snapped _returnvalue_3 _returnvalue))
  (bind _returnvalue_5 (Math|Vector|Lerp(Vector) _returnvalue_4 _returnvalue_2 0.5))
  (Variables|Default|SetMoving true)
  (if (Variables|Default|GetSnapped)
    (Transformation|SetWorldLocation (Variables|Default|GetSphere) _returnvalue_5 false false)
    (else
      (Transformation|SetActorLocation _returnvalue_5 false false))))

(event EventReturn
  (bind _returnvalue (Utilities|Time|SetTimerbyEvent (delegate Custom|MoveDown) 0.001 true))
  (bind _output_get (Variables|Default|SetMoving false))
  (CallFunction|Release _output_get))

(fn ConstructionScript)

(fn DoThing
  (params (Angle :type Float%20%28double-precision%29) (Press :type Boolean))
  (bind _output_get (Variables|Default|SetPressed Press))
  (Transformation|SetRelativeRotation (Variables|Default|GetLighter) (Math|Rotator|Lerp(Rotator) (Variables|/Script/Engine.SceneComponent|GetRelativeRotation (Variables|Default|GetLighter)) (select _output_get "0.000000,0.000000,-180.000000" "0, 0, 0") 0.2 true) false false)
  (return))

(fn GetRotation
  (return (Variables|Default|GetAngle)))