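; Level 2 volcano bucket that simulates a timed 30-second pour, draining its contents while a second fill level rises.
; Start runs a looping timer shifting StartAmount into CurAmount, with Niagara flow, dust and faded audio, and marks Tutorial steps at start and end.
; Tick and construction trace the top and bottom edges to set a dynamic material's world height, raise the Cube and feed its transform to that material.
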(event Custom|Start
  (bind _audio2 (Variables|Default|GetAudio2))
  (Utilities|FlowControl|DoOnce false
    (:Completed
      (Utilities|FlowControl|Sequence
        (:then_0
          (Utilities|Time|SetTimerbyEvent (delegate Custom|Stop) 3e+01)
          (bind _returnvalue (Utilities|Time|SetTimerbyEvent (delegate Custom|Reduce) 0.01 true))
          (Components|Activation|Activate (Variables|Default|GetNiagara) false)
          (Components|Activation|Activate _audio2 false)
          (bind _volume (Timeline|Timeline_0 Play)
            (:Update
              (Audio|Components|Audio|SetVolumeMultiplier _audio2 _volume :!class /Script/Engine.AudioComponent))))
        (:then_1
          (bind _foundwidgets (Widget|GetAllWidgetsOfClass "/Game/Blueprints/UI/Tutorial.Tutorial_C" true))
          (Class|StepCheckInterface|Mark(Message) (Utilities|Array|Get(acopy) _foundwidgets) 0 "NewEnumerator1"))))))

(event Custom|Stop
  (bind _audio2 (Variables|Default|GetAudio2))
  (Utilities|Time|ClearandInvalidateTimerbyHandle (stale Custom|Start _returnvalue))
  (Variables|Default|SetRate 0.0)
  (bind _volume (Timeline|Timeline Play)
    (:Update
      (Audio|Components|Audio|SetVolumeMultiplier _audio2 _volume :!class /Script/Engine.AudioComponent))
    (:Finished
      (Components|Activation|Deactivate _audio2)
      (bind _foundwidgets (Widget|GetAllWidgetsOfClass "/Game/Blueprints/UI/Tutorial.Tutorial_C" true))
      (Class|StepCheckInterface|Mark(Message) (Utilities|Array|Get(acopy) _foundwidgets) 1 "NewEnumerator1"))))

(event Custom|Reduce
  (Variables|Default|SetStartAmount (Math|Float|Clamp(Float) (- (Variables|Default|GetStartAmount) 0.001) 0.0 (Variables|Default|GetStartAmountInit)))
  (Variables|Default|SetCurAmount (Math|Float|Clamp(Float) (+ (Variables|Default|GetCurAmount) 0.0056) 0.0 (Variables|Default|GetMaxAmount)))
  (Variables|Default|SetRate (Math|Float|Lerp (Variables|Default|GetRate) (* (/ (Variables|Default|GetStartAmount) (Variables|Default|GetStartAmountInit)) 5e+03) 0.02)))

(event Custom|CustomEvent)

(event Custom|Starting%20In
  (Variables|Default|SetTimer (- (Variables|Default|GetTimer) 0.3))
  (Development|PrintString (Utilities|String|Append "Starting in: " (Utilities|String|ToString(Float) (Variables|Default|GetTimer)))))

(event EventBeginPlay
  (CallFunction|InitMaterial))

(event EventTick
  (params (DeltaSeconds :type Float%20%28single-precision%29))
  (CallFunction|Ray)
  (CallFunction|CountHeight)
  (CallFunction|SetMaterial)
  (CallFunction|CubeHeight)
  (CallFunction|NiagaraSetup))

(fn ConstructionScript
  (Utilities|FlowControl|Sequence
    (:then_0
      (Utilities|FlowControl|DoOnce false
        (:Completed
          (CallFunction|InitMaterial))))
    (:then_1
      (CallFunction|Ray)
      (CallFunction|CountHeight)
      (CallFunction|SetMaterial)
      (CallFunction|CubeHeight)
      (CallFunction|NiagaraSetup))))

(fn SetMaterial
  (bind _material (Variables|Default|GetMaterial))
  (Rendering|Material|SetScalarParameterValue _material "Height" (/ (Variables|Default|GetHeight) 0.01) :!class /Script/Engine.MaterialInstanceDynamic)
  (Rendering|Material|SetScalarParameterValue _material "Fade" 0.01 :!class /Script/Engine.MaterialInstanceDynamic)
  (Rendering|Material|SetVectorParameterValue _material "ColorUp" (Variables|Default|GetColorUp) :!class /Script/Engine.MaterialInstanceDynamic)
  (Rendering|Material|SetVectorParameterValue _material "ColorDown" (Variables|Default|GetColorDown) :!class /Script/Engine.MaterialInstanceDynamic))

(fn InitMaterial
  (bind _returnvalue (Rendering|Material|CreateDynamicMaterialInstance "/Game/Blueprints/Level2/2_HeightMat_Inst.2_HeightMat_Inst" "2_1" "None" :!class /Script/Engine.KismetMaterialLibrary))
  (bind _output_get (Variables|Default|SetMaterial _returnvalue))
  (Rendering|Material|SetMaterial (Variables|Default|GetStaticMesh1) 0 _output_get))

(fn Ray
  (bind _array (Utilities|Array|MakeArray "ObjectTypeQuery2"))
  (bind _downpoint (Variables|Default|GetDownPoint))
  (bind _uppoint (Variables|Default|GetUpPoint))
  (bind _returnvalue (Transformation|GetWorldLocation _downpoint))
  (bind _returnvalue_2 (Transformation|GetWorldLocation _uppoint))
  (Utilities|FlowControl|Sequence
    (:then_0
      (bind _outhit (Collision|LineTraceForObjects _returnvalue_2 (+ _returnvalue_2 (* (Transformation|GetActorUpVector) -2e+01)) _array false 0 "None" false))
      (Variables|Default|SetUpEdge (.z (.Location (Collision|BreakHitResult _outhit)))))
    (:then_1
      (bind _outhit_2 (Collision|LineTraceForObjects _returnvalue (+ _returnvalue (* (Transformation|GetActorUpVector) 2e+01)) _array false 0 "None" false))
      (Variables|Default|SetDownEdge (.z (.Location (Collision|BreakHitResult _outhit_2)))))))

(fn CountHeight
  (bind _downedge (Variables|Default|GetDownEdge))
  (Variables|Default|SetHeight (* (+ (* (- (Variables|Default|GetUpEdge) _downedge) (/ (Variables|Default|GetStartAmount) (Variables|Default|GetMaxAmount))) _downedge) -1.0)))

(fn CubeHeight
  (bind _cube (Variables|Default|GetCube))
  (bind _maxamount (Variables|Default|GetMaxAmount))
  (bind _curamount (Variables|Default|GetCurAmount))
  (bind _material (Variables|Default|GetMaterial))
  (bind _returnvalue (Transformation|GetWorldTransform _cube))
  (bind _returnvalue_2 (/ _curamount _maxamount))
  (bind _returnvalue_3 (Math|Float|Lerp 6.15 16.5 _returnvalue_2))
  (Transformation|SetRelativeLocation (Variables|Default|GetCube) (Math|Vector|MakeVector 0.0 0.0 _returnvalue_3) false false)
  (Transformation|SetRelativeLocation (Variables|Default|GetNiagara) (Math|Vector|MakeVector 0.0 0.0 (- _returnvalue_3 6.35)) false false)
  (Rendering|Material|SetVectorParameterValue _material "Location" (Math|Conversions|ToLinearColor(Vector) (.location _returnvalue)) :!class /Script/Engine.MaterialInstanceDynamic)
  (Rendering|Material|SetVectorParameterValue _material "Scale" (Math|Conversions|ToLinearColor(Vector) (.scale _returnvalue)) :!class /Script/Engine.MaterialInstanceDynamic))

(fn NiagaraSetup
  (bind _rate (Variables|Default|GetRate))
  (Niagara|SetNiagaraVariable(Float) (Variables|Default|GetNiagara) "Rate" _rate)
  (Niagara|SetNiagaraVariable(Float) (Variables|Default|Get2_Volcano_Dust) "Rate" (/ _rate 5.0)))