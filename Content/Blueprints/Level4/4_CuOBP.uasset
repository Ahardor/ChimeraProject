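; Level 4 liquid container child Blueprint (CuO, by its name) that animates a change once a second compound is present.
; Gated Start and Stop events drive height and color timelines, tinting that compound blue and fading audio.
; Parent overrides scale Niagara spilling and draining by tilt angle, depleting each compound.
; A dynamic material draws two color layers split at the animated height, while the surface cylinder tracks fill level.
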(event Custom|Start
  (bind _audio2 (Variables|Default|GetAudio2))
  (bind _audio2_2 (Variables|Default|GetAudio2))
  (Utilities|FlowControl|Gate true
    (:Exit
      (Variables|Default|SetStarted true)
      (Utilities|FlowControl|Sequence
        (:then_0
          (bind _heightalpha (Timeline|HeightTimeLine Play)
            (:Update
              (Utilities|FlowControl|Sequence
                (:then_0
                  (bind _output_get (Variables|Default|SetHeight%20Alpha _heightalpha))
                  (Utilities|Struct|SetmembersinCompound (Utilities|Array|Get(acopy) (Variables|Default|GetCompound) 1) (Math|Color|Lerp(LinearColor) "(R=0.000000,G=0.196078,B=0.486275,A=0.000000)" "(R=0.000000,G=0.196078,B=0.486275,A=0.479000)" _heightalpha)))
                (:then_1
                  (bind _color (Timeline|ColorTimeLine Play)
                    (:Update
                      (Variables|Default|SetColor _color))))))))
        (:then_1
          (Components|Activation|Activate _audio2_2 false)
          (bind _volume (Timeline|Timeline Play)
            (:Update
              (Audio|Components|Audio|SetVolumeMultiplier _audio2_2 _volume :!class /Script/Engine.AudioComponent))))
        (:then_2
          (bind _volume_2 (Timeline|Timeline_0 SetNewTime)
            (:Update
              (Audio|Components|Audio|SetVolumeMultiplier _audio2 _volume_2 :!class /Script/Engine.AudioComponent))
            (:Finished
              (Components|Activation|Deactivate _audio2))))))))

(event Custom|CanStart
  (params (? :type Boolean))
  (bind _audio2 (Variables|Default|GetAudio2))
  (bind _audio2_2 (Variables|Default|GetAudio2))
  (if ?
    (Utilities|FlowControl|Gate true) ; enters at Open
    (else
      (Utilities|FlowControl|Gate true) ; enters at Close
    )))

(event Custom|Stop
  (bind _audio2 (Variables|Default|GetAudio2))
  (Variables|Default|SetStarted false)
  (Utilities|FlowControl|Sequence
    (:then_0
      (bind _heightalpha (Timeline|HeightTimeLine Stop)
        (:Update
          (Utilities|FlowControl|Sequence
            (:then_0
              (bind _output_get (Variables|Default|SetHeight%20Alpha _heightalpha))
              (Utilities|Struct|SetmembersinCompound (Utilities|Array|Get(acopy) (Variables|Default|GetCompound) 1) (Math|Color|Lerp(LinearColor) "(R=0.000000,G=0.196078,B=0.486275,A=0.000000)" "(R=0.000000,G=0.196078,B=0.486275,A=0.479000)" _heightalpha)))
            (:then_1
              (bind _color (Timeline|ColorTimeLine Play)
                (:Update
                  (Variables|Default|SetColor _color))))))))
    (:then_1
      (Timeline|ColorTimeLine Stop))
    (:then_2
      (bind _volume (Timeline|Timeline_0 Play)
        (:Update
          (Audio|Components|Audio|SetVolumeMultiplier _audio2 _volume :!class /Script/Engine.AudioComponent))
        (:Finished
          (Components|Activation|Deactivate _audio2))))
    (:then_3
      (bind _volume_2 (Timeline|Timeline SetNewTime)
        (:Update
          (Audio|Components|Audio|SetVolumeMultiplier (Variables|Default|GetAudio2) _volume_2 :!class /Script/Engine.AudioComponent))))))

(event EventBeginPlay
  (|CallParentFunction) ; This node is disabled and will not be called.\nDrag off pins to build functionality.
)

(event Collision|EventActorBeginOverlap
  (params (OtherActor :type Actor%20Object%20Reference))
  (|CallParentFunction OtherActor) ; This node is disabled and will not be called.\nDrag off pins to build functionality.
)

(event EventTick
  (params (DeltaSeconds :type Float%20%28single-precision%29))
  (|CallParentFunction DeltaSeconds)
  (Utilities|FlowControl|Sequence
    (:then_0
      (if (> (Utilities|Array|Length (Variables|Default|GetCompound)) 1)
        (Utilities|FlowControl|DoOnce false
          (:Completed
            (CallFunction|Start)
            (Variables|Default|SetbCanStart true)
            (Variables|Default|SetHeight%20Alpha 1.0)))))))

(fn ConstructionScript
  (|CallParentFunction))

(fn Spill
  (bind _compound (Variables|Default|GetCompound))
  (bind _minspillrate (Variables|Default|GetMinSpillRate))
  (bind _maxspillrate (Variables|Default|GetMaxSpillRate))
  (bind _angle (Variables|Default|GetAngle))
  (bind _niagara (Variables|Default|GetNiagara))
  (bind _returnvalue (Math|Float|Absolute(Float) _angle))
  (bind _returnvalue_2 (/ _returnvalue 9e+01))
  (bind _returnvalue_3 (Math|Float|Lerp _minspillrate _maxspillrate _returnvalue_2))
  (if (!= (Variables|Default|GetFill) 0.0)
    (Effects|Components|ParticleSystem|SetFloatParameter _niagara "SpawnRate" (Math|Float|Lerp 1e+01 (* (Variables|Default|GetMaxSpillRadius) 3e+03) _returnvalue_2))
    (Effects|Components|ParticleSystem|SetFloatParameter _niagara "SpawnRadius" (Math|Float|Lerp 0.2 (Variables|Default|GetMaxSpillRadius) _returnvalue_2))
    (bind _output_get (Variables|Default|SetSpillPoint (Math|Vector|Lerp(Vector) (Transformation|GetWorldLocation (Variables|Default|GetParticleInit)) (- (/ (+ (Transformation|GetWorldLocation (Variables|Default|GetCube1)) (Transformation|GetWorldLocation (Variables|Default|GetCube2))) 2.0) (Variables|Default|GetParticleOffset)) (Math|Float|Clamp(Float) (/ (- _returnvalue 9e+01) 9e+01)))))
    (Transformation|SetWorldLocation (Variables|Default|GetNiagara) _output_get false false)
    (bind _output_get_2 (Variables|Default|SetSpillRate _returnvalue_3))
    (bind _output_get_3 (Variables|Default|SetFill (Math|Float|Clamp(Float) (- (Variables|Default|GetFill) _returnvalue_3) 0.0 (Variables|Default|GetMaxFill))))
    (for (_ _array_index) _compound
      (Utilities|Struct|SetmembersinCompound (Utilities|Array|Get(acopy) _compound _array_index) (Math|Float|Clamp(Float) (- (.Amount (Utilities|Struct|BreakCompound (Utilities|Array|Get(acopy) _compound _array_index))) (/ _output_get_2 (Utilities|Array|Length _compound))) 0.0 (Variables|Default|GetMaxFill)))
      (if (== (Math|Float|Clamp(Float) (- (.Amount (Utilities|Struct|BreakCompound (Utilities|Array|Get(acopy) _compound _array_index))) (/ _output_get_2 (Utilities|Array|Length _compound))) 0.0 (Variables|Default|GetMaxFill)) 0.0)
        (Utilities|Array|RemoveIndex _compound _array_index)))
    (if (== _output_get_3 0.0)
      (Rendering|SetVisibility (Variables|Default|GetStaticMesh1) false false))))

(fn ComputeColor
  (Variables|Default|SetColor (Variables|Default|GetColor)))

(fn SetMPCParams
  (bind _returnvalue (Transformation|GetActorLocation))
  (bind _compound (Variables|Default|GetCompound))
  (bind _downpoint (Variables|Default|GetDownPoint))
  (bind _compound_2 (Variables|Default|GetCompound))
  (bind _cube (Variables|Default|GetCube))
  (bind _staticmesh1 (Variables|Default|GetStaticMesh1))
  (bind _returnvalue_2 (Transformation|GetWorldTransform _cube))
  (bind _returnvalue_3 (Rendering|Material|CreateDynamicMaterialInstance _staticmesh1 0 (Rendering|Material|GetMaterial _staticmesh1 0) "None" :!class /Script/Engine.PrimitiveComponent))
  (Utilities|FlowControl|Sequence
    (:then_0
      (Utilities|FlowControl|DoOnce false
        (:Completed
          (Rendering|Material|SetMaterial (Variables|Default|GetCylinder) 0 _returnvalue_3))))
    (:then_1
      (Rendering|Material|SetVectorParameterValue _returnvalue_3 "Location" (Math|Conversions|ToLinearColor(Vector) (.location _returnvalue_2)) :!class /Script/Engine.MaterialInstanceDynamic)
      (Rendering|Material|SetVectorParameterValue _returnvalue_3 "Scale" (Math|Conversions|ToLinearColor(Vector) (.scale _returnvalue_2)) :!class /Script/Engine.MaterialInstanceDynamic)
      (Rendering|Material|SetVectorParameterValue _returnvalue_3 "ColorUp" (Variables|Default|GetColor) :!class /Script/Engine.MaterialInstanceDynamic)
      (Rendering|Material|SetVectorParameterValue _returnvalue_3 "ColorDown" (select (> (Utilities|Array|Length _compound_2) 1) (.color (Utilities|Array|Get(acopy) _compound_2 1)) "") :!class /Script/Engine.MaterialInstanceDynamic)
      (Rendering|Material|SetScalarParameterValue _returnvalue_3 "Height" (Variables|Default|GetHeight) :!class /Script/Engine.MaterialInstanceDynamic)
      (Transformation|SetWorldLocation (Variables|Default|GetCylinder) (Math|Vector|MakeVector (.x _returnvalue) (.y _returnvalue) (- (Math|Float|Lerp (Variables|Default|GetDownPoint) (Variables|Default|GetUpPoint) (/ (Variables|Default|GetFill) (Variables|Default|GetMaxFill))) 1.0)) false false)
      (if (> (Utilities|Array|Length _compound) 1)
        (Variables|Default|SetHeight (Math|Float|Lerp (* _downpoint -99.0) (* (Math|Float|Lerp _downpoint (Variables|Default|GetUpPoint) (/ (.amount (Utilities|Array|Get(acopy) _compound 1)) (Variables|Default|GetMaxFill))) -1e+02) (Variables|Default|GetHeight%20Alpha)))))))