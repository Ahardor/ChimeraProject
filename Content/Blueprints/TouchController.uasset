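; Touch controller that lets the player pick up, drag, rotate and release BaseInteractionActor, Dropper and Spoon objects through interface messages.
; A Touch1 press stores the traced actor and opens a gate, which the Touch axis drives to move it to a PhysicsBody line-trace hit while easing rotation toward zero.
; RotationTouch switches to rotation from horizontal cursor offset.
; Release sends Spoons to the Bucket, Droppers to the DropperBase and others slightly downward.
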(event Custom|RotateActor
  (bind (_locationx _locationy) (Game|Player|GetMousePosition))
  (bind _hitactor (Variables|Default|GetHitActor))
  (Utilities|IsValid _hitactor
    (:Is%20Valid
      (Utilities|FlowControl|Sequence
        (:then_0
          (Utilities|FlowControl|DoOnce false
            (:Completed
              (Variables|Default|SetStartXLoc _locationx)
              (Variables|Default|SetStartYLoc _locationy))))
        (:then_1
          (Class|InteractionInterface|Rotate(Message) _hitactor (Math|Float|Lerp 0.0 1.8e+02 (Math|Float|Clamp(Float) (/ (- _locationx (Variables|Default|GetStartXLoc)) 5e+02) -1.0)) true))))))

(event Custom|ResetRotating
  (bind (_locationx _locationy) (Game|Player|GetMousePosition))
  (Utilities|FlowControl|DoOnce false) ; enters at Reset
)

(event Input|ActionEvents|InputActionRotationTouch
  (params (Key :type Key%20Structure :default "None"))
  (:Pressed
    (Utilities|IsValid (Variables|Default|GetHitActor)
      (:Is%20Valid
        (Variables|Default|SetisRotating true))))
  (:Released
    (Variables|Default|SetisRotating false)
    (CallFunction|ResetRotating)))

(event Input|AxisEvents|InputAxisTouch
  (params (AxisValue :type Float%20%28single-precision%29))
  (bind _returnvalue (Game|Player|GetPlayerPawn 0))
  (bind _returnvalue_2 (Transformation|GetActorLocation _returnvalue))
  (if (Variables|Default|GetisRotating)
    (CallFunction|RotateActor)
    (else
      (Utilities|FlowControl|Gate true
        (:Exit
          (Utilities|IsValid (stale Input|TouchEvents|Touch1 _output_get)
            (:Is%20Valid
              (bind _outhit (Collision|LineTraceForObjects (- _returnvalue_2 "0.000000,0.000000,10.000000") (+ (* (.WorldDirection (Game|Player|ConvertMouseLocationToWorldSpace)) 5e+02) _returnvalue_2) (Utilities|Array|MakeArray "ObjectTypeQuery4") false 0 "None"))
              (Class|InteractionInterface|Move(Message) (stale Input|TouchEvents|Touch1 _output_get) (.Location (Collision|BreakHitResult _outhit)))
              (bind _angle (Class|InteractionInterface|GetRotation(Message) (stale Input|TouchEvents|Touch1 _output_get)))
              (Class|InteractionInterface|Rotate(Message) (stale Input|TouchEvents|Touch1 _output_get) (Math|Float|Lerp _angle 0.0 0.2) false))))))))

(event Input|AxisEvents|InputAxisScroll
  (params (AxisValue :type Float%20%28single-precision%29))
  (Utilities|IsValid (Variables|Default|GetHitActor)
    (:Is%20Valid
      (Variables|Default|SetDistance (+ (Variables|Default|GetDistance) AxisValue)))))

(event Input|TouchEvents|Touch1
  (params (Key :type Key%20Structure :default "None"))
  (bind _hitresult (Class|PlayerController|GetHitResultUnderFingerbyChannel "Touch1" "TraceTypeQuery1" true))
  (bind _returnvalue (Game|Player|GetPlayerPawn 0))
  (bind (_bblockinghit _binitialoverlap _time _distance _location _impactpoint _normal _impactnormal _physmat _hitactor) (Collision|BreakHitResult _hitresult))
  (bind _returnvalue_2 (Transformation|GetActorLocation _returnvalue))
  (:Pressed
    (if _bblockinghit
      (if (Math|Boolean|ORBoolean (Class|GameplayStatics|ObjectIsA _hitactor "/Game/Blueprints/BaseInteractionActor.BaseInteractionActor_C") (Class|GameplayStatics|ObjectIsA _hitactor "/Game/Blueprints/Dropper.Dropper_C") (Class|GameplayStatics|ObjectIsA _hitactor "/Game/Blueprints/Spoon.Spoon_C"))
        (Utilities|FlowControl|Sequence
          (:then_0
            (bind _output_get (Variables|Default|SetHitActor _hitactor))
            (Variables|Default|SetDistance (.x (Transformation|GetActorLocation _output_get))))
          (:then_1
            (Utilities|FlowControl|Gate true) ; enters at Open
          )))))
  (:Released
    (Utilities|FlowControl|Sequence
      (:then_0
        (Utilities|FlowControl|Gate true) ; enters at Close
      )
      (:then_1
        (Variables|Default|SetDistance 0.0)
        (Utilities|IsValid (Variables|Default|GetHitActor)
          (:Is%20Valid
            (bind _output_get_2 (Variables|Default|SetInitLoc (Transformation|GetActorLocation (Variables|Default|GetHitActor))))
            (bind _outactors (Actor|GetAllActorsOfClass "/Game/Blueprints/DropperBase.DropperBase_C"))
            (bind _outactors_2 (Actor|GetAllActorsOfClass "/Game/Blueprints/Bucket.Bucket_C"))
            (Class|InteractionInterface|Return(Message) (Variables|Default|GetHitActor) (select (Class|GameplayStatics|ObjectIsA (Variables|Default|GetHitActor) "/Game/Blueprints/Spoon.Spoon_C") (Transformation|GetActorLocation (Utilities|Array|Get(acopy) _outactors_2)) (select (Class|GameplayStatics|ObjectIsA (Variables|Default|GetHitActor) "/Game/Blueprints/Dropper.Dropper_C") (Transformation|GetActorLocation (Utilities|Array|Get(acopy) _outactors)) (- _output_get_2 "0.000000,0.000000,20.000000"))))
            (Variables|Default|SetHitActor 0)))))))

(fn ConstructionScript)

(fn GetRotation
  (return 0.0))

(fn Rotate
  (params (Angle :type Float%20%28double-precision%29) (Press :type Boolean))
  (return))