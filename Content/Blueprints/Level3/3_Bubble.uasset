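; Level 3 container Blueprint that bubbles when its Compound array holds more than one entry, marking Tutorial steps.
; Tick drives bubble Niagara and timeline-faded audio, marking one step as bubbling starts and another after the fade-out.
; While bubbling, it calls an overridden Spill that drains Fill and compound amounts at an Angle-based rate and moves the spill particles.
; ComputeColor is overridden to leave Color unchanged.
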(event EventBeginPlay
  (|CallParentFunction) ; This node is disabled and will not be called.\nDrag off pins to build functionality.
)

(event Collision|EventActorBeginOverlap
  (params (OtherActor :type Actor%20Object%20Reference))
  (|CallParentFunction OtherActor) ; This node is disabled and will not be called.\nDrag off pins to build functionality.
)

(event EventTick
  (params (DeltaSeconds :type Float%20%28single-precision%29))
  (bind _niagara1 (Variables|Default|GetNiagara1))
  (bind _audio2 (Variables|Default|GetAudio2))
  (bind _niagara1_2 (Variables|Default|GetNiagara1))
  (bind _audio2_2 (Variables|Default|GetAudio2))
  (|CallParentFunction DeltaSeconds)
  (Utilities|FlowControl|Sequence
    (:then_0
      (if (> (Utilities|Array|Length (Variables|Default|GetCompound)) 1)
        (Utilities|FlowControl|Sequence
          (:then_0
            (Components|Activation|Activate _niagara1 false)
            (Components|Activation|Activate _audio2_2 false)
            (bind _volume (Timeline|Timeline Play)
              (:Update
                (Audio|Components|Audio|SetVolumeMultiplier _audio2_2 _volume :!class /Script/Engine.AudioComponent)
                (Variables|Default|SetStarted true))))
          (:then_1
            (Utilities|FlowControl|DoOnce false
              (:Completed
                (bind _foundwidgets (Widget|GetAllWidgetsOfClass "/Game/Blueprints/UI/Tutorial.Tutorial_C" true))
                (Class|StepCheckInterface|Mark(Message) (Utilities|Array|Get(acopy) _foundwidgets) 0 "NewEnumerator1")))))
        (else
          (Components|Activation|Deactivate _niagara1)
          (if (Variables|Default|GetStarted)
            (bind _volume_2 (Timeline|Timeline_0 Play)
              (:Update
                (Audio|Components|Audio|SetVolumeMultiplier _audio2 _volume_2 :!class /Script/Engine.AudioComponent))
              (:Finished
                (Components|Activation|Deactivate _audio2)
                (bind _foundwidgets_2 (Widget|GetAllWidgetsOfClass "/Game/Blueprints/UI/Tutorial.Tutorial_C" true))
                (Class|StepCheckInterface|Mark(Message) (Utilities|Array|Get(acopy) _foundwidgets_2) 1 "NewEnumerator1")))))))
    (:then_1
      (if (Components|Activation|IsActive _niagara1_2)
        (if (!= (Variables|Default|GetFill) 0.0)
          (CallFunction|Spill)
          (else
            (Components|Activation|Deactivate _niagara1_2)
            (Utilities|Array|Clear (Variables|Default|GetCompound))))))))

(fn ConstructionScript
  (|CallParentFunction))

(fn Spill
  (bind _compound (Variables|Default|GetCompound))
  (bind _minspillrate (Variables|Default|GetMinSpillRate))
  (bind _maxspillrate (Variables|Default|GetMaxSpillRate))
  (bind _angle (Variables|Default|GetAngle))
  (bind _niagara (Variables|Default|GetNiagara))
  (bind _returnvalue (Math|Float|Absolute(Float) _angle))
  (bind _returnvalue_2 (/ _returnvalue 9e+01))
  (bind _returnvalue_3 (Math|Float|Lerp _minspillrate _maxspillrate _returnvalue_2))
  (if (!= (Variables|Default|GetFill) 0.0)
    (Effects|Components|ParticleSystem|SetFloatParameter _niagara "SpawnRate" (Math|Float|Lerp 1e+01 (* (Variables|Default|GetMaxSpillRadius) 3e+03) _returnvalue_2))
    (Effects|Components|ParticleSystem|SetFloatParameter _niagara "SpawnRadius" (Math|Float|Lerp 0.2 (Variables|Default|GetMaxSpillRadius) _returnvalue_2))
    (bind _output_get (Variables|Default|SetSpillPoint (Math|Vector|Lerp(Vector) (Transformation|GetWorldLocation (Variables|Default|GetParticleInit)) (- (/ (+ (Transformation|GetWorldLocation (Variables|Default|GetCube1)) (Transformation|GetWorldLocation (Variables|Default|GetCube2))) 2.0) (Variables|Default|GetParticleOffset)) (Math|Float|Clamp(Float) (/ (- _returnvalue 9e+01) 9e+01)))))
    (Transformation|SetWorldLocation (Variables|Default|GetNiagara) _output_get false false)
    (bind _output_get_2 (Variables|Default|SetSpillRate _returnvalue_3))
    (bind _output_get_3 (Variables|Default|SetFill (Math|Float|Clamp(Float) (- (Variables|Default|GetFill) _returnvalue_3) 0.0 (Variables|Default|GetMaxFill))))
    (for (_ _array_index) _compound
      (Utilities|Struct|SetmembersinCompound (Utilities|Array|Get(acopy) _compound _array_index) (Math|Float|Clamp(Float) (- (.Amount (Utilities|Struct|BreakCompound (Utilities|Array|Get(acopy) _compound _array_index))) (/ _output_get_2 (Utilities|Array|Length _compound))) 0.0 (Variables|Default|GetMaxFill)))
      (if (== (Math|Float|Clamp(Float) (- (.Amount (Utilities|Struct|BreakCompound (Utilities|Array|Get(acopy) _compound _array_index))) (/ _output_get_2 (Utilities|Array|Length _compound))) 0.0 (Variables|Default|GetMaxFill)) 0.0)
        (Utilities|Array|RemoveIndex _compound _array_index)))
    (if (== _output_get_3 0.0)
      (Rendering|SetVisibility (Variables|Default|GetStaticMesh1) false false))))

(fn ComputeColor
  (Variables|Default|SetColor (Variables|Default|GetColor)))